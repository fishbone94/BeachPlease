(event `self.ReceiveBeginPlay`
  ;[1 1 1] Get PlayerPawn and cast to BP_Player for later use
  (bind _asbp_player (cast `/Game/BP_Player` (`GameplayStatics.GetPlayerPawn` 0)))
  (set `self.BP_Player` _asbp_player)
  (bind _asbp_game_state (cast `/Game/BP_GameState` (`GameplayStatics.GetGameState`)))
  (set `self.BPGameState` _asbp_game_state))

(event `InputAxisKey|MouseX`
  (params (AxisValue :type "Float (single-precision)"))
  (bind _bp_player (`self.BP_Player`))
  (bind _returnvalue (/ (`self.GetMousePosition`) (`KismetMathLibrary.BreakVector2D` (`WidgetLayoutLibrary.GetViewportSize`))))
  ;[1 1 1] Edge Pan
  (if (> _returnvalue 0.95)
    (`/Game/BP_Player.PanRight` _bp_player 1.0)
    (elif (< _returnvalue 0.05)
      (`/Game/BP_Player.PanRight` _bp_player -1.0))))

(event `InputAxisKey|MouseY`
  (params (AxisValue :type "Float (single-precision)"))
  (bind _bp_player (`self.BP_Player`))
  (bind _returnvalue (/ (`.LocationY` (`self.GetMousePosition`)) (`.Y` (`KismetMathLibrary.BreakVector2D` (`WidgetLayoutLibrary.GetViewportSize`)))))
  ;[1 1 1] Edge Pan
  (if (> _returnvalue 0.95)
    (`/Game/BP_Player.PanUp` _bp_player -1.0)
    (elif (< _returnvalue 0.05)
      (`/Game/BP_Player.PanUp` _bp_player 1.0))))

(event `EnterBuildMode`
  ;[1 1 1] Enter Build Mode spawns ghost towers
  (set `self.IsBuildMode` true)
  (bind _outactors (`GameplayStatics.GetAllActorsOfClass` "/Game/Towers/BP_GhostParent.BP_GhostParent_C"))
  (for _array_element _outactors
    (`self.K2_DestroyActor` _array_element))
  (switch `/Game/Towers/BP_TowerList` (`self.TowerToBuild`)
    (:`NewEnumerator0`
      (set `self.WhichGhost` "/Game/Towers/BP_GhostTowerA.BP_GhostTowerA_C"))
    (:`NewEnumerator1`
      (set `self.WhichGhost` "/Game/Towers/BP_GhostTowerB.BP_GhostTowerB_C"))
    (:`NewEnumerator2`
      (set `self.WhichGhost` "/Game/Towers/BP_GhostTowerC.BP_GhostTowerC_C"))
    (:`NewEnumerator3`
      (set `self.WhichGhost` "/Game/Towers/BP_GhostWall.BP_GhostWall_C")))
  (bind _returnvalue (`|SpawnActorFromClass` (`self.WhichGhost`) (`KismetMathLibrary.MakeTransform` (0.0 0.0 0.0)) "Undefined" "OverrideRootScale"))
  (set `self.GhostComponent` _returnvalue))

(event `ExitBuildMode`
  ;[1 1 1] Exit Build Mode
  (set `self.IsBuildMode` false)
  (bind _outactors (`GameplayStatics.GetAllActorsOfClass` "/Game/Towers/BP_GhostParent.BP_GhostParent_C"))
  (for _array_element _outactors
    (`self.K2_DestroyActor` _array_element)))

(event `Key|RightMouseButton`
  (params (Key :type "Key Structure" :default "AnyKey"))
  ;[1 1 1] Cancel Tower Placement
  (:`Pressed`
    (if (`self.IsBuildMode`)
      (`self.ExitBuildMode`))))

(event `Key|LeftMouseButton`
  (params (Key :type "Key Structure" :default "AnyKey"))
  (bind _bpgamestate (`self.BPGameState`))
  ;[1 1 1] Place towers
  (:`Pressed`
    (if (`self.IsBuildMode`)
      (bind _asbp_ghost_parent (cast `/Game/Towers/BP_GhostParent` (`self.GhostComponent`)))
      (if (not (`/Game/Towers/BP_GhostParent.isOverlap` _asbp_ghost_parent))
        (switch `/Game/Towers/BP_TowerList` (`self.TowerToBuild`)
          (:`NewEnumerator0`
            (set `self.WhichTower` "/Game/Towers/BP_TowerA.BP_TowerA_C")
            (`/Game/BP_GameState.ChangePlayerSeashells` _bpgamestate -50))
          (:`NewEnumerator1`
            (set `self.WhichTower` "/Game/Towers/BP_TowerB.BP_TowerB_C")
            (`/Game/BP_GameState.ChangePlayerSeashells` _bpgamestate -100))
          (:`NewEnumerator2`
            (set `self.WhichTower` "/Game/Towers/BP_TowerC.BP_TowerC_C")
            (`/Game/BP_GameState.ChangePlayerSeashells` _bpgamestate -200))
          (:`NewEnumerator3`
            (set `self.WhichTower` "/Game/Towers/BP_Wall.BP_Wall_C")
            (`/Game/BP_GameState.ChangePlayerSeashells` _bpgamestate -25)))
        (`|SpawnActorFromClass` (`self.WhichTower`) (`KismetMathLibrary.Conv_VectorToTransform` (`.Location` (`GameplayStatics.BreakHitResult` (`self.GetHitResultUnderCursorForObjects` (`|MakeArray` "ObjectTypeQuery1" :!type "EObjectTypeQuery Enum"))))) "Undefined" "OverrideRootScale")
        (`self.ExitBuildMode`)))))

(fn `UserConstructionScript`)