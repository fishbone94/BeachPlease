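; BP_EndTarget is the goal that enemies try to reach, costing the player a life for each one that arrives.
; It caches BP_GameState on BeginPlay, then uses its sphere's begin overlap to detect actors derived from BP_EnemyParent.
; Each such enemy has its name printed, decrements PlayerLives and is destroyed, with GameOver called on the game state when lives equal zero.
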(event `self.ReceiveBeginPlay`
  (bind _asbp_game_state (cast `/Game/BP_GameState` (`GameplayStatics.GetGameState`)))
  (set `self.BP_GameState` _asbp_game_state))

(event `self.Sphere.OnComponentBeginOverlap`
  (params (OverlappedComponent :type "PrimitiveComponent Object Reference") (OtherActor :type "Actor Object Reference") (OtherComp :type "PrimitiveComponent Object Reference") (OtherBodyIndex :type Integer) (bFromSweep :type Boolean) (SweepResult :type "HitResult Structure (by ref)"))
  (bind _bp_gamestate (`self.BP_GameState`))
  (bind _playerlives (`/Game/BP_GameState.PlayerLives` _bp_gamestate))
  (if (`KismetMathLibrary.ClassIsChildOf` (`GameplayStatics.GetObjectClass` OtherActor) "/Game/Enemies/BP_EnemyParent.BP_EnemyParent_C")
    (`KismetSystemLibrary.PrintString` (`KismetSystemLibrary.GetDisplayName` OtherActor))
    (set `/Game/BP_GameState.PlayerLives` (- _playerlives 1) _bp_gamestate)
    (`self.K2_DestroyActor` OtherActor)
    (if (== _playerlives 0)
      (`/Game/BP_GameState.GameOver` _bp_gamestate))))

(fn `UserConstructionScript`)