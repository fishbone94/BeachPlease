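; BP_Player is a top-down style camera actor with mouse-wheel zoom and planar panning.
; UpdateCamera places the camera on a sphere around the actor from radius and two angles, aimed at the center, on construction and each zoom.
; PanUp and PanRight move the actor along the camera's yaw-only axes, adding edge-axis values to input, scaled by speed without delta time.
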(event `Key|MouseScrollUp`
  (params (Key :type "Key Structure" :default "AnyKey"))
  ;[1 1 1] Zoom
  (:`Pressed`
    (set `self.CameraRadius` (`KismetMathLibrary.FClamp` (- (`self.CameraRadius`) (`self.ZoomSpeed`)) (`self.RadiusMin`) (`self.RadiusMax`)))
    (`self.UpdateCamera` :!label _label)))

(event `Key|MouseScrollDown`
  (params (Key :type "Key Structure" :default "AnyKey"))
  ;[1 1 1] Zoom
  (:`Pressed`
    (set `self.CameraRadius` (`KismetMathLibrary.FClamp` (+ (`self.CameraRadius`) (`self.ZoomSpeed`)) (`self.RadiusMin`) (`self.RadiusMax`)))
    (goto _label)))

(fn `PanRight`
  (params (Axis :type "Float (double-precision)"))
  (`self.K2_SetActorLocation` (+ (* (`KismetMathLibrary.GetRightVector` (`KismetMathLibrary.MakeRotator` 0.0 0.0 (.yaw (`SceneComponent.K2_GetComponentRotation` (`self.Camera`))))) (* (+ Axis (`self.EdgeRightAxis`)) (`self.MovementSpeed`))) (`self.K2_GetActorLocation`))))

(fn `PanUp`
  (params (Axis :type "Float (double-precision)"))
  (`self.K2_SetActorLocation` (+ (* (`KismetMathLibrary.GetForwardVector` (`KismetMathLibrary.MakeRotator` 0.0 0.0 (.yaw (`SceneComponent.K2_GetComponentRotation` (`self.Camera`))))) (* (+ Axis (`self.EdgeForwardAxis`)) (`self.MovementSpeed`))) (`self.K2_GetActorLocation`))))

(fn `UpdateCamera`
  (bind _camera (`self.Camera`))
  (bind _cameraradius (`self.CameraRadius`))
  (bind _camerazangle (`self.CameraZAngle`))
  (bind _cameraheightangle (`self.CameraHeightAngle`))
  ;[1 1 1] Update camera location each time this function is called
  (`SceneComponent.K2_SetRelativeLocation` _camera (`KismetMathLibrary.MakeVector` (* _cameraradius (`KismetMathLibrary.DegCos` _camerazangle) (`KismetMathLibrary.DegSin` _cameraheightangle)) (* _cameraradius (`KismetMathLibrary.DegSin` _camerazangle) (`KismetMathLibrary.DegSin` _cameraheightangle)) (* _cameraradius (`KismetMathLibrary.DegCos` _cameraheightangle))) false false)
  (`SceneComponent.K2_SetRelativeRotation` _camera (`KismetMathLibrary.FindLookAtRotation` (`SceneComponent.RelativeLocation` _camera) (`KismetMathLibrary.MakeVector` 0.0)) false false))

(fn `UserConstructionScript`
  (`self.UpdateCamera`))