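; BP_GameState drives wave progression, tracks the player's seashell count and opens the Game_Over level on game over.
; On BeginPlay it starts the background music and caches a BP_EnemySpawn, keeping only the last one found.
; Tick polls for remaining BP_EnemyParent actors and, when none remain, increments the wave number and starts a countdown.
; A delayed-loop macro steps that countdown, which calls SpawnWave on the cached spawner at zero.
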(event `self.ReceiveBeginPlay`
  (bind _outactors (`GameplayStatics.GetAllActorsOfClass` "/Game/Enemies/BP_EnemySpawn.BP_EnemySpawn_C"))
  (for _array_element _outactors
    (set `self.BP_EnemySpawn` _array_element)
    (`AudioComponent.Play` (`self.BGM`) 0.0)))

(event `self.ReceiveTick`
  (params (DeltaSeconds :type "Float (single-precision)"))
  ;[1 1 1] Countdown is no enemies left on the map
  (if (not (`self.IsCountingDown`))
    (bind _outactors (`GameplayStatics.GetAllActorsOfClass` "/Game/Enemies/BP_EnemyParent.BP_EnemyParent_C"))
    (if (== (`KismetArrayLibrary.Array_Length` _outactors) 0)
      (`/Engine/EditorBlueprintResources/StandardMacros.IncrementInt` (`self.WaveNumber`)
        (:`  `
          (set `self.TimeUntilNextWave` 5.0)
          (`self.Countdown`))))))

(event `Countdown`
  ;[1 1 1] Countdown timer until next wave
  (set `self.IsCountingDown` true)
  (`self.LoopWithDelay` 0 4 1.0
    (:`LoopBody`
      (bind _output_get (set `self.TimeUntilNextWave` (- (`self.TimeUntilNextWave`) 1.0)))
      (if (== _output_get 0.0)
        (set `self.IsCountingDown` false)
        (`/Game/Enemies/BP_EnemySpawn.SpawnWave` (`self.BP_EnemySpawn`))))))

(event `GameOver`
  (`GameplayStatics.OpenLevel` "Game_Over"))

(fn `ChangePlayerSeashells`
  (params (Seashells :type Integer))
  (set `self.PlayerSeashells` (+ Seashells (`self.PlayerSeashells`))))

(fn `UserConstructionScript`)