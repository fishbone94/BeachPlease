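; Base tower Actor that automatically shoots enemies in range and can be clicked for editing.
; Radius collision overlaps maintain a target list; Tick yaws the turret toward the first entry and spawns projectiles carrying that target and tower damage, throttled by a Delay-based cooldown.
; Clicking base or turret toggles its widget, hiding other tower and wall widgets when showing it, and registers the tower with the player controller for edit mode.
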(event `self.ReceiveBeginPlay`
  (bind _asbp_player_controller (cast `/Game/BP_PlayerController` (`GameplayStatics.GetPlayerController` 0)))
  (set `self.BP_PlayerController` _asbp_player_controller))

(event `self.TowerRadiusCollision.OnComponentBeginOverlap`
  (params (OverlappedComponent :type "PrimitiveComponent Object Reference") (OtherActor :type "Actor Object Reference") (OtherComp :type "PrimitiveComponent Object Reference") (OtherBodyIndex :type Integer) (bFromSweep :type Boolean) (SweepResult :type "HitResult Structure (by ref)"))
  ;[1 1 1] Track Enemies within Radius(Collision)
  (if (`KismetMathLibrary.ClassIsChildOf` (`GameplayStatics.GetObjectClass` OtherActor) "/Game/Enemies/BP_EnemyParent.BP_EnemyParent_C")
    (bind _asbp_enemy_parent (cast `/Game/Enemies/BP_EnemyParent` OtherActor))
    (`KismetArrayLibrary.Array_Add` (`self.target_list`) _asbp_enemy_parent)))

(event `self.TowerRadiusCollision.OnComponentEndOverlap`
  (params (OverlappedComponent :type "PrimitiveComponent Object Reference") (OtherActor :type "Actor Object Reference") (OtherComp :type "PrimitiveComponent Object Reference") (OtherBodyIndex :type Integer))
  ;[1 1 1] Track Enemies within Radius(Collision)
  (if (`KismetMathLibrary.ClassIsChildOf` (`GameplayStatics.GetObjectClass` OtherActor) "/Game/Enemies/BP_EnemyParent.BP_EnemyParent_C")
    (bind _asbp_enemy_parent (cast `/Game/Enemies/BP_EnemyParent` OtherActor))
    (`KismetArrayLibrary.Array_RemoveItem` (`self.target_list`) _asbp_enemy_parent)))

(event `self.ReceiveTick`
  (params (DeltaSeconds :type "Float (single-precision)"))
  (bind _staticmeshturret (`self.StaticMeshTurret`))
  (bind _item (`KismetArrayLibrary.Array_Get` (`self.target_list`)))
  ;[1 1 1] Auto shooting projectiles
  (if (`KismetSystemLibrary.IsValid` _item)
    (`|ExecutionSequence`
      (:`then_0`
        ;[1 1 1] Rotate turret to enemy
        (`SceneComponent.K2_SetRelativeRotation` _staticmeshturret (`KismetMathLibrary.RInterpTo` (`SceneComponent.RelativeRotation` _staticmeshturret) (`KismetMathLibrary.MakeRotator` 0.0 0.0 (+ (.yaw (`KismetMathLibrary.FindLookAtRotation` (`self.K2_GetActorLocation`) (`self.K2_GetActorLocation` _item))) -90.0)) (`GameplayStatics.GetWorldDeltaSeconds`) 20.0) false false))
      (:`then_1`
        (if (not (`self.IsInternalCoolDown`))
          (set `self.IsInternalCoolDown` true)
          (bind _returnvalue (`|SpawnActorFromClass` "/Game/Towers/BP_basicProjectiles.BP_basicProjectiles_C" (`KismetMathLibrary.MakeTransform` (`KismetMathLibrary.MakeVector` (.x (`self.K2_GetActorLocation`)) (.y (`self.K2_GetActorLocation`)) (+ (.z (`self.K2_GetActorLocation`)) 130.0)) (`self.K2_GetActorRotation` _item)) "AlwaysSpawn" "OverrideRootScale"))
          (`AudioComponent.Play` (`self.Shooting`) 0.0)
          (set `/Game/Towers/BP_basicProjectiles.targetEnemy` _item _returnvalue)
          (set `/Game/Towers/BP_basicProjectiles.ProjectileDamage` (`self.TowerDamage`) _returnvalue)
          (`KismetSystemLibrary.Delay` (`self.TowerAtkSpeed`))
          (set `self.IsInternalCoolDown` false))))))

(event `self.StaticMeshBase.OnClicked`
  (params (TouchedComponent :type "PrimitiveComponent Object Reference") (ButtonPressed :type "Key Structure" :default "AnyKey"))
  (bind _bp_playercontroller (`self.BP_PlayerController`))
  (bind _widget (`self.Widget`))
  (if (`SceneComponent.IsVisible` (`self.Widget`)) :!label _label
    (`SceneComponent.SetVisibility` _widget false false)
    (set `/Game/BP_PlayerController.IsTowerEditMode` true _bp_playercontroller :!label _label_2)
    (set `/Game/BP_PlayerController.TowerToEdit` self _bp_playercontroller)
    (else
      (bind _outactors (`GameplayStatics.GetAllActorsOfClass` "BP_TowerParent_C"))
      (for _array_element _outactors
        (`SceneComponent.SetVisibility` (`/Game/Towers/BP_TowerParent.Widget` _array_element) false false)
        (bind _outactors_2 (`GameplayStatics.GetAllActorsOfClass` "/Game/Towers/BP_Wall.BP_Wall_C"))
        (if (`KismetArrayLibrary.Array_IsValidIndex` _outactors_2)
          (for _array_element_2 _outactors_2
            (`SceneComponent.SetVisibility` (`/Game/Towers/BP_Wall.Widget` _array_element_2) false false)
            (`SceneComponent.SetVisibility` _widget true false :!label _label_3)
            (goto _label_2))
          (else
            (goto _label_3)))))))

(event `self.StaticMeshTurret.OnClicked`
  (params (TouchedComponent :type "PrimitiveComponent Object Reference") (ButtonPressed :type "Key Structure" :default "AnyKey"))
  (goto _label))

(fn `UserConstructionScript`)