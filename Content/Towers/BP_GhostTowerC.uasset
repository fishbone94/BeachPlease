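; BP_GhostTowerC is a ghost tower that tints its turret mesh to show whether it is overlapping.
; The construction script creates a dynamic material instance on the turret mesh and stores it as TurretOverlap.
; Each Tick calls the parent, then sets that material's Color to translucent red when IsOverlap is true, otherwise green.
; IsOverlap is only read here, and the overlap event is empty.
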(event `self.ReceiveActorBeginOverlap`
  (params (OtherActor :type "Actor Object Reference")))

(event `self.ReceiveTick`
  (params (DeltaSeconds :type "Float (single-precision)"))
  (bind _turretoverlap (`self.TurretOverlap`))
  (`parent.ReceiveTick` 0.0)
  (if (`self.isOverlap`)
    (`MaterialInstanceDynamic.SetVectorParameterValue` _turretoverlap "Color" (struct :`R` 1.0 :`A` 0.5))
    (else
      (`MaterialInstanceDynamic.SetVectorParameterValue` _turretoverlap "Color" (struct :`R` 0.019408 :`G` 1.0 :`A` 0.5)))))

(fn `UserConstructionScript`
  (`parent.UserConstructionScript`)
  (bind _returnvalue (`PrimitiveComponent.CreateDynamicMaterialInstance` (`self.StaticMeshTurret`) 0 null))
  (set `self.TurretOverlap` _returnvalue))