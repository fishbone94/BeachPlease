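; BP_GhostWall is a placement preview wall that follows the mouse cursor for tower and wall building.
; Every tick it moves to the location of a world-static trace under the cursor, using the player controller cached on BeginPlay.
; Its cube's overlap events set an IsOverlap flag when touching components tagged TowerBase, tracking whether it intersects other towers or walls.
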(event `self.ReceiveBeginPlay`
  (bind _asbp_player_controller (cast `/Game/BP_PlayerController` (`GameplayStatics.GetPlayerController` 0)))
  (set `self.PlayerController` _asbp_player_controller)
  (bind _asbp_player (cast `/Game/BP_Player` (`GameplayStatics.GetPlayerPawn` 0)))
  (set `self.PlayerPawn` _asbp_player))

(event `self.ReceiveTick`
  (params (DeltaSeconds :type "Float (single-precision)"))
  ;[1 1 1] Make ghost walls follow cursor
  (`self.K2_SetActorLocation` (`.Location` (`GameplayStatics.BreakHitResult` (`PlayerController.GetHitResultUnderCursorForObjects` (`self.PlayerController`) (`|MakeArray` "ObjectTypeQuery1" :!type "EObjectTypeQuery Enum") true)))))

(event `self.Cube.OnComponentBeginOverlap`
  (params (OverlappedComponent :type "PrimitiveComponent Object Reference") (OtherActor :type "Actor Object Reference") (OtherComp :type "PrimitiveComponent Object Reference") (OtherBodyIndex :type Integer) (bFromSweep :type Boolean) (SweepResult :type "HitResult Structure (by ref)"))
  ;[1 1 1] Check for overlap with other towers and walls
  (if (`ActorComponent.ComponentHasTag` OtherComp "TowerBase")
    (set `self.isOverlap` true)))

(event `self.Cube.OnComponentEndOverlap`
  (params (OverlappedComponent :type "PrimitiveComponent Object Reference") (OtherActor :type "Actor Object Reference") (OtherComp :type "PrimitiveComponent Object Reference") (OtherBodyIndex :type Integer))
  ;[1 1 1] Check for overlap with other towers and walls
  (if (`ActorComponent.ComponentHasTag` OtherComp "TowerBase")
    (set `self.isOverlap` false)))

(fn `UserConstructionScript`)