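; BP_basicProjectiles is a homing tower projectile that damages enemies on contact.
; BeginPlay enables strong homing on its projectile movement and destroys the actor after a three-second lifetime.
; Each Tick re-points homing at the capsule of the assigned TargetEnemy while it is valid.
; A sphere overlap with any BP_EnemyParent subclass applies ProjectileDamage, then destroys the projectile.
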(event `self.ReceiveBeginPlay`
  (bind _projectilemovement (`self.ProjectileMovement`))
  (set `ProjectileMovementComponent.bIsHomingProjectile` true _projectilemovement)
  (set `ProjectileMovementComponent.HomingAccelerationMagnitude` 10000.0 _projectilemovement)
  ;[1 1 1] destroy self after 3s
  (`KismetSystemLibrary.Delay` 3.0)
  (`self.K2_DestroyActor`))

(event `self.ReceiveTick`
  (params (DeltaSeconds :type "Float (single-precision)"))
  (bind _targetenemy (`self.targetEnemy`))
  ;[1 1 1] set homing projectiles
  (if (`KismetSystemLibrary.IsValid` _targetenemy)
    (set `ProjectileMovementComponent.HomingTargetComponent` (`Character.CapsuleComponent` _targetenemy) (`self.ProjectileMovement`))))

(event `self.Sphere.OnComponentBeginOverlap`
  (params (OverlappedComponent :type "PrimitiveComponent Object Reference") (OtherActor :type "Actor Object Reference") (OtherComp :type "PrimitiveComponent Object Reference") (OtherBodyIndex :type Integer) (bFromSweep :type Boolean) (SweepResult :type "HitResult Structure (by ref)"))
  (if (`KismetMathLibrary.ClassIsChildOf` (`GameplayStatics.GetObjectClass` OtherActor) "/Game/Enemies/BP_EnemyParent.BP_EnemyParent_C")
    (bind _asbp_enemy_parent (cast `/Game/Enemies/BP_EnemyParent` OtherActor))
    (`/Game/Enemies/BP_EnemyParent.TakeDamage` _asbp_enemy_parent (`self.ProjectileDamage`))
    (`self.K2_DestroyActor`)))

(fn `UserConstructionScript`)