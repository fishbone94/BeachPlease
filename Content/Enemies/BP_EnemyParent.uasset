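; Parent enemy for a tower-defense style game that walks toward the BP_EndTarget and pays out seashells when killed.
; Tick re-issues the move to the target and turns a scene component toward the player's camera.
; When its velocity is near zero, it destroys any walls and towers close by to clear blockages.
; Damage updates the health bar widget, and death awards loot through the game state before destroying the enemy.
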(event `self.ReceiveBeginPlay`
  ;[1 1 1] Set End Target
  (`AudioComponent.Play` (`self.SpawnSound`) 0.0)
  (bind _outactors (`GameplayStatics.GetAllActorsOfClass` "/Game/Other/BP_EndTarget.BP_EndTarget_C"))
  (for _array_element _outactors
    (set `self.EndTarget` _array_element)
    (bind _asbp_game_state (cast `/Game/BP_GameState` (`GameplayStatics.GetGameState`)))
    (set `self.BP_GameState` _asbp_game_state)
    (set `self.EnemyMaxHealth` (`self.EnemyHealth`))
    (bind _asbp_player (cast `/Game/BP_Player` (`GameplayStatics.GetPlayerPawn` 0)))
    (set `self.BP_player` _asbp_player)))

(event `self.ReceiveTick`
  (params (DeltaSeconds :type "Float (single-precision)"))
  (bind _scene (`self.Scene`))
  ;[1 1 1] Lets Enemy Move to End Target
  (`NavigationSystem.SimpleMoveToLocation` (`self.GetController`) (`self.K2_GetActorLocation` (`self.EndTarget`)))
  (`SceneComponent.K2_SetWorldRotation` _scene (`KismetMathLibrary.FindLookAtRotation` (`SceneComponent.K2_GetComponentLocation` _scene) (`SceneComponent.K2_GetComponentLocation` (`/Game/BP_Player.Camera` (`self.BP_player`)))) false false)
  ;[1 1 1] Kill towers and walls that block off
  (if (== (`MovementComponent.Velocity` (`self.CharacterMovement`)) (0.0 0.0 0.0))
    (bind _outactors (`GameplayStatics.GetAllActorsOfClass` "/Game/Towers/BP_Wall.BP_Wall_C"))
    (for _array_element _outactors
      (if (<= (`self.GetDistanceTo` _array_element self) 150.0)
        (`self.K2_DestroyActor` _array_element)))
    (bind _outactors_2 (`GameplayStatics.GetAllActorsOfClass` "/Game/Towers/BP_TowerParent.BP_TowerParent_C"))
    (for _array_element_2 _outactors_2
      (if (<= (`self.GetDistanceTo` _array_element_2 self) 150.0)
        (`self.K2_DestroyActor` _array_element_2)))))

(event `TakeDamage`
  (params (Damage :type Integer))
  ;[1 1 1] Take Damage
  (bind _output_get (set `self.EnemyHealth` (- (`self.EnemyHealth`) Damage)))
  (bind _asbp_enemy_health (cast `/Game/UI/BP_EnemyHealth` (`WidgetComponent.GetUserWidgetObject` (`self.Widget`))))
  (`ProgressBar.SetPercent` (`/Game/UI/BP_EnemyHealth.ProgressBar_460` _asbp_enemy_health) (/ (`KismetMathLibrary.Conv_IntToDouble` (`self.EnemyHealth`)) (`KismetMathLibrary.Conv_IntToDouble` (`self.EnemyMaxHealth`))))
  (if (<= _output_get 0)
    (`/Game/BP_GameState.ChangePlayerSeashells` (`self.BP_GameState`) (`self.EnemyLoot`))
    (`AudioComponent.Play` (`self.MoneySound`) 0.0)
    (`self.K2_DestroyActor`)))

(fn `UserConstructionScript`)