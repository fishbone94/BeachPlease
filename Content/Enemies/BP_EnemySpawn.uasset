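; Enemy spawner actor that releases a timed wave of enemies at its own location when SpawnWave is called.
; SpawnWave reads WaveNumber from BP_GameState, cached on BeginPlay, choosing fish, crab or turtle, with turtles also covering any later or unmatched wave.
; Each wave uses the LoopWithDelay macro, a for-loop with a delay between iterations, to stagger spawns and give each enemy its default controller.
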(event `self.ReceiveBeginPlay`
  (bind _asbp_game_state (cast `/Game/BP_GameState` (`GameplayStatics.GetGameState`)))
  (set `self.BP_GameState` _asbp_game_state))

(event `SpawnWave`
  (switch `int` (`/Game/BP_GameState.WaveNumber` (`self.BP_GameState`))
    (:`Default`
      (`self.SpawnWave3` :!label _label))
    (:`1`
      (`self.SpawnWave1`))
    (:`2`
      (`self.SpawnWave2`))
    (:`3`
      (goto _label))))

(event `SpawnWave1`
  (`self.LoopWithDelay` 0 5 1.5
    (:`LoopBody`
      (bind _returnvalue (`|SpawnActorFromClass` "/Game/Enemies/BP_EnemyFish.BP_EnemyFish_C" (`KismetMathLibrary.MakeTransform` (`self.K2_GetActorLocation`)) "AdjustIfPossibleButAlwaysSpawn" "OverrideRootScale"))
      (`Pawn.SpawnDefaultController` _returnvalue))))

(event `SpawnWave2`
  (`self.LoopWithDelay` 0 5 1.5
    (:`LoopBody`
      (bind _returnvalue (`|SpawnActorFromClass` "/Game/Enemies/BP_EnemyCrab.BP_EnemyCrab_C" (`KismetMathLibrary.MakeTransform` (`self.K2_GetActorLocation`)) "AdjustIfPossibleButAlwaysSpawn" "OverrideRootScale"))
      (`Pawn.SpawnDefaultController` _returnvalue))))

(event `SpawnWave3`
  (`self.LoopWithDelay` 0 5 1.5
    (:`LoopBody`
      (bind _returnvalue (`|SpawnActorFromClass` "/Game/Enemies/BP_EnemyTurtle.BP_EnemyTurtle_C" (`KismetMathLibrary.MakeTransform` (`self.K2_GetActorLocation`)) "AdjustIfPossibleButAlwaysSpawn" "OverrideRootScale"))
      (`Pawn.SpawnDefaultController` _returnvalue))))

(fn `UserConstructionScript`)